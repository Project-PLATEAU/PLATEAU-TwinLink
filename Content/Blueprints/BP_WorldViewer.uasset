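; Player-controlled TwinLink world viewer that handles camera movement, building and urban-planning clicks, and asset placement editing.
; Enhanced Input events forward movement and look values to movement functions and drive the placement functions.
; In placement mode, Tick traces under the cursor to move the unsettled actor until input release settles it.
; In transform mode, TwinLinkTransformer selects and edits assets, toggling translation and rotation, with edits and removals reported to the placement system.
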(event `self.ReceiveBeginPlay`
  (bind _asplayer_controller (cast `PlayerController` (`self.GetController`)))
  (message `EnhancedInputSubsystemInterface.AddMappingContext` (pcsubsystem `EnhancedInputLocalPlayerSubsystem` _asplayer_controller) "/PLATEAU-TwinLink/Input/Mappings/IMC_WorldViewer_KBM.IMC_WorldViewer_KBM" 0 (struct))
  ;[1 1 1] アセット配置機能セットアップ
  (`TwinLinkTransformerComponent.SetSpaceType` (`self.TwinLinkTransformer`) "ST_Local"))

(event `EnhancedInput|/PLATEAU-TwinLink/Input/Actions/IA_MoveForward`
  (params (ActionValue :type "Float (double-precision)") (ElapsedSeconds :type "Float (double-precision)") (TriggeredSeconds :type "Float (double-precision)") (InputAction :type "InputAction Object Reference" :default "/PLATEAU-TwinLink/Input/Actions/IA_MoveForward.IA_MoveForward"))
  (:`Triggered`
    (`self.MoveForward` ActionValue)))

(event `EnhancedInput|/PLATEAU-TwinLink/Input/Actions/IA_MoveForward_Mouse`
  (params (ActionValue :type "Float (double-precision)") (ElapsedSeconds :type "Float (double-precision)") (TriggeredSeconds :type "Float (double-precision)") (InputAction :type "InputAction Object Reference" :default "/PLATEAU-TwinLink/Input/Actions/IA_MoveForward_Mouse.IA_MoveForward_Mouse"))
  (:`Triggered`
    (`self.MoveForward` ActionValue)))

(event `self.ReceiveTick`
  (params (DeltaSeconds :type "Float (single-precision)"))
  (`self.AssetPlacementTick`))

(event `EnhancedInput|/PLATEAU-TwinLink/Input/Actions/IA_MoveRight_Mouse`
  (params (ActionValue :type "Float (double-precision)") (ElapsedSeconds :type "Float (double-precision)") (TriggeredSeconds :type "Float (double-precision)") (InputAction :type "InputAction Object Reference" :default "/PLATEAU-TwinLink/Input/Actions/IA_MoveRight_Mouse.IA_MoveRight_Mouse"))
  (:`Triggered`
    (`self.MoveRight` ActionValue)))

(event `EnhancedInput|/PLATEAU-TwinLink/Input/Actions/IA_MoveRight`
  (params (ActionValue :type "Float (double-precision)") (ElapsedSeconds :type "Float (double-precision)") (TriggeredSeconds :type "Float (double-precision)") (InputAction :type "InputAction Object Reference" :default "/PLATEAU-TwinLink/Input/Actions/IA_MoveRight.IA_MoveRight"))
  (:`Triggered`
    (`self.MoveRight` ActionValue)))

(event `EnhancedInput|/PLATEAU-TwinLink/Input/Actions/IA_ActivateControlViewMovement`
  (params (ActionValue :type Boolean) (ElapsedSeconds :type "Float (double-precision)") (TriggeredSeconds :type "Float (double-precision)") (InputAction :type "InputAction Object Reference" :default "/PLATEAU-TwinLink/Input/Actions/IA_ActivateControlViewMovement.IA_ActivateControlViewMovement"))
  (:`Started`
    (`self.AssetPlacementSelect`))
  (:`Completed`
    (`self.AssetPlacementComplete`)))

(event `EnhancedInput|/PLATEAU-TwinLink/Input/Actions/IA_MoveUp`
  (params (ActionValue :type "Float (double-precision)") (ElapsedSeconds :type "Float (double-precision)") (TriggeredSeconds :type "Float (double-precision)") (InputAction :type "InputAction Object Reference" :default "/PLATEAU-TwinLink/Input/Actions/IA_MoveUp.IA_MoveUp"))
  (:`Triggered`
    (`self.MoveUp` ActionValue)))

(event `EnhancedInput|/PLATEAU-TwinLink/Input/Actions/IA_Turn`
  (params (ActionValue :type "Float (double-precision)") (ElapsedSeconds :type "Float (double-precision)") (TriggeredSeconds :type "Float (double-precision)") (InputAction :type "InputAction Object Reference" :default "/PLATEAU-TwinLink/Input/Actions/IA_Turn.IA_Turn"))
  (:`Triggered`
    (`self.Turn` ActionValue)))

(event `EnhancedInput|/PLATEAU-TwinLink/Input/Actions/IA_ActivateControlViewAngle`
  (params (ActionValue :type Boolean) (ElapsedSeconds :type "Float (double-precision)") (TriggeredSeconds :type "Float (double-precision)") (InputAction :type "InputAction Object Reference" :default "/PLATEAU-TwinLink/Input/Actions/IA_ActivateControlViewAngle.IA_ActivateControlViewAngle"))
  (:`Started`
    (`self.AssetPlacementSwitchTransformation`)))

(event `EnhancedInput|/PLATEAU-TwinLink/Input/Actions/IA_LookUp`
  (params (ActionValue :type "Float (double-precision)") (ElapsedSeconds :type "Float (double-precision)") (TriggeredSeconds :type "Float (double-precision)") (InputAction :type "InputAction Object Reference" :default "/PLATEAU-TwinLink/Input/Actions/IA_LookUp.IA_LookUp"))
  (:`Triggered`
    (`self.LookUp` ActionValue)))

(event `EnhancedInput|/PLATEAU-TwinLink/Input/Actions/IA_AssetPlacementRemove`
  (params (ActionValue :type Boolean) (ElapsedSeconds :type "Float (double-precision)") (TriggeredSeconds :type "Float (double-precision)") (InputAction :type "InputAction Object Reference" :default "/PLATEAU-TwinLink/Input/Actions/IA_AssetPlacementRemove.IA_AssetPlacementRemove"))
  (:`Completed`
    (`self.AssetPlacementRemove`)))

(event `EnhancedInput|/PLATEAU-TwinLink/Input/Actions/IA_Click_Building`
  (params (ActionValue :type Boolean) (ElapsedSeconds :type "Float (double-precision)") (TriggeredSeconds :type "Float (double-precision)") (InputAction :type "InputAction Object Reference" :default "/PLATEAU-TwinLink/Input/Actions/IA_Click_Building.IA_Click_Building"))
  (:`Triggered`
    (`self.Click`)
    (`TwinLinkUrbanPlanningViewSystem.TwinLinkSelectUrbanPlanning` (subsystem `TwinLinkUrbanPlanningViewSystem`))))

(fn `AssetPlacementComplete`
  (bind _twinlinktransformer (`self.TwinLinkTransformer`))
  (if (`self.EnableAssetPlacement`)
    (switch `ETwinLinkAssetPlacementModes` (`TwinLinkAssetPlacementSystem.TwinLinkAssetPlacementGetMode` (subsystem `TwinLinkAssetPlacementSystem`))
      (:`AssetPlacement`
        (`TwinLinkAssetPlacementSystem.TwinLinkAssetPlacementSettledActor` (subsystem `TwinLinkAssetPlacementSystem`))
        (bind _foundwidgets (`WidgetBlueprintLibrary.GetAllWidgetsOfClass` "/PLATEAU-TwinLink/Widgets/MapEdit/WBP_TwinLinkAssetPlacementElement.WBP_TwinLinkAssetPlacementElement_C" false))
        (for _array_element _foundwidgets
          (`Widget.SetVisibility` (`/PLATEAU-TwinLink/Widgets/MapEdit/WBP_TwinLinkAssetPlacementElement.AssetPlacementButtonFrameImage` _array_element) "Hidden")))
      (:`AssetTransform`
        (`TwinLinkTransformerComponent.ClearDomain` _twinlinktransformer)
        (bind _asactor (cast `Actor` (`KismetSystemLibrary.GetOuterObject` (`|GetArrayItem` (`TwinLinkTransformerComponent.GetSelectedComponents` _twinlinktransformer)))))
        (`TwinLinkAssetPlacementSystem.TwinLinkAssetPlacementUpdateActor` (subsystem `TwinLinkAssetPlacementSystem`) _asactor)))))

(fn `AssetPlacementRemove`
  (bind _outcomponentlist (`TwinLinkTransformerComponent.GetSelectedComponents` (`self.TwinLinkTransformer`)))
  (bind _returnvalue (`ActorComponent.GetOwner` (`|GetArrayItem` _outcomponentlist)))
  (if (`KismetMathLibrary.Conv_IntToBool` (`KismetArrayLibrary.Array_Length` _outcomponentlist))
    (if (`KismetStringLibrary.StartsWith` (`KismetSystemLibrary.GetObjectName` _returnvalue) "StaticMeshActor")
      (bind _output_get (set `self.RemoveActor` _returnvalue))
      (`TwinLinkTransformerComponent.DeselectAll` (`self.TwinLinkTransformer`) false)
      (`TwinLinkAssetPlacementSystem.TwinLinkAssetPlacementRemoveActor` (subsystem `TwinLinkAssetPlacementSystem`) _output_get)
      (`self.K2_DestroyActor` _output_get))))

(fn `AssetPlacementSelect`
  (if (`self.EnableAssetPlacement`)
    (switch `ETwinLinkAssetPlacementModes` (`TwinLinkAssetPlacementSystem.TwinLinkAssetPlacementGetMode` (subsystem `TwinLinkAssetPlacementSystem`))
      (:`AssetTransform`
        (bind _returnvalue (`TwinLinkBlueprintLibrary.TwinLinkGetCityModel`))
        (bind _returnvalue_2 (`TwinLinkBlueprintLibrary.TwinLinkGetFacilityModel`))
        (`TwinLinkTransformerComponent.MouseTraceByObjectTypes` (`self.TwinLinkTransformer`) 5000000.0 (`|MakeArray` "ECC_WorldStatic" "ECC_WorldDynamic" :!type "ECollisionChannel Enum") (`|MakeArray` _returnvalue_2 _returnvalue) false)))))

(fn `AssetPlacementTick`
  (bind _returnvalue (subsystem `TwinLinkAssetPlacementSystem`))
  (bind (_worldlocation _worlddirection) (`PlayerController.DeprojectMousePositionToWorld` (`GameplayStatics.GetPlayerController` 0)))
  (if (`self.EnableAssetPlacement`)
    (switch `ETwinLinkAssetPlacementModes` (`TwinLinkAssetPlacementSystem.TwinLinkAssetPlacementGetMode` _returnvalue)
      (:`AssetPlacement`
        (bind (_outhit _returnvalue_2) (`KismetSystemLibrary.LineTraceSingle` _worldlocation (+ _worldlocation (* _worlddirection 300000.0)) "TraceTypeQuery1" false (`|MakeArray` (`TwinLinkAssetPlacementSystem.TwinLinkAssetPlacementGetUnsettledActor` _returnvalue))))
        (if _returnvalue_2
          (`TwinLinkAssetPlacementSystem.TwinLinkAssetPlacementUpdateUnsettledActor` (subsystem `TwinLinkAssetPlacementSystem`) (`.Location` (`GameplayStatics.BreakHitResult` _outhit))))))))

(fn `UserConstructionScript`)