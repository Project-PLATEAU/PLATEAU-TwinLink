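; TwinLinkUIColorLib is a Blueprint function library that supplies UI text colors by theme.
; GetSlateColorFromTextTheme switches on a text theme enum (Standard, Warning, Error, Complete) and returns a matching fixed Slate color: off-white, yellow, red or green.
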(fn `GetSlateColorFromTextTheme`
  (params (Theme :type "/PLATEAU-TwinLink/Blueprints/TwinLinkUITextColTheme Enum" :default "NewEnumerator3"))
  (returns (Color :type "SlateColor Structure"))
  (locals (NewLocalVar :type "SlateColor Structure"))
  (switch `/PLATEAU-TwinLink/Blueprints/TwinLinkUITextColTheme` Theme
    (:`NewEnumerator3`
      (set `local.NewLocalVar` (make `SlateColor` (struct :`R` 0.932292 :`G` 0.932292 :`B` 0.932292 :`A` 1.0))))
    (:`NewEnumerator0`
      (set `local.NewLocalVar` (make `SlateColor` (struct :`R` 0.932292 :`G` 0.774125 :`A` 1.0))))
    (:`NewEnumerator1`
      (set `local.NewLocalVar` (make `SlateColor` (struct :`R` 0.932292 :`B` 0.120996 :`A` 1.0))))
    (:`NewEnumerator2`
      (set `local.NewLocalVar` (make `SlateColor` (struct :`G` 1.0 :`B` 0.261789 :`A` 1.0)))))
  (return (`local.NewLocalVar`)))