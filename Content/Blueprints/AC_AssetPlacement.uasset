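; Actor component for BP_TwinLink that sets up TwinLink asset placement and its selection UI.
; On BeginPlay it registers the owner's Vehicle and Prop preset assets with the TwinLink asset placement system, then triggers relocation of assets.
; ShowWidget spawns an actor and opens the placement panel, filling separate Vehicle and Prop wrap boxes with one element widget per preset, each set up by preset ID.
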(event `self.ReceiveBeginPlay`
  (bind _returnvalue (subsystem `TwinLinkAssetPlacementSystem`))
  (bind _asbp_twin_link (cast `/PLATEAU-TwinLink/Blueprints/BP_TwinLink` (`self.GetOwner`)))
  ;[1 1 1] プリセットアセット登録（Vehicle）
  (for _array_element (`/PLATEAU-TwinLink/Blueprints/BP_TwinLink.PresetAssets_Vehicle` _asbp_twin_link)
    (`TwinLinkAssetPlacementSystem.TwinLinkAssetPlacementRegistPresetAsset` _returnvalue _array_element))
  ;[1 1 1] プリセットアセット登録（Prop）
  (for _array_element_2 (`/PLATEAU-TwinLink/Blueprints/BP_TwinLink.PresetAssets_Prop` _asbp_twin_link)
    (`TwinLinkAssetPlacementSystem.TwinLinkAssetPlacementRegistPresetAsset` _returnvalue _array_element_2))
  ;[1 1 1] アセット再配置
  (`TwinLinkAssetPlacementSystem.TwinLinkAssetPlacementRelocation` _returnvalue))

(event `ShowWidget`
  (`|SpawnActorFromClass` "/PLATEAU-TwinLink/Blueprints/BP_TransformerPawn.BP_TransformerPawn_C" (`KismetMathLibrary.MakeTransform` (0.0 0.0 0.0)) "Undefined" "MultiplyWithRoot" null null)
  (bind _returnvalue (`|CreateWidget` "/PLATEAU-TwinLink/Widgets/WBP_TwinLinkAssetPlacementPanel.WBP_TwinLinkAssetPlacementPanel_C"))
  (`UserWidget.AddToViewport` _returnvalue 0)
  ;[1 1 1] プリセットアセットウィジェット生成（Vehicle）
  (for _array_element (`/PLATEAU-TwinLink/Blueprints/BP_TwinLink.PresetAssets_Vehicle` (stale `self.ReceiveBeginPlay` _asbp_twin_link))
    (bind _returnvalue_2 (`|CreateWidget` "/PLATEAU-TwinLink/Widgets/WBP_TwinLinkAssetPlacementElement.WBP_TwinLinkAssetPlacementElement_C"))
    (`WrapBox.AddChildToWrapBox` (`/PLATEAU-TwinLink/Widgets/WBP_TwinLinkAssetPlacementPanel.AssetPlacementWrapBox_Vehicle` _returnvalue) _returnvalue_2)
    (`TwinLinkAssetPlacementElement.TwinLinkAssetPlacementElementSetup` _returnvalue_2 (`.PresetID` (break `TwinLinkAssetPlacementPresetData` _array_element)) (`/PLATEAU-TwinLink/Widgets/WBP_TwinLinkAssetPlacementElement.AssetPlacementButton` _returnvalue_2)))
  ;[1 1 1] プリセットアセットウィジェット生成（Prop）
  (for _array_element_2 (`/PLATEAU-TwinLink/Blueprints/BP_TwinLink.PresetAssets_Prop` (stale `self.ReceiveBeginPlay` _asbp_twin_link))
    (bind _returnvalue_3 (`|CreateWidget` "/PLATEAU-TwinLink/Widgets/WBP_TwinLinkAssetPlacementElement.WBP_TwinLinkAssetPlacementElement_C"))
    (`WrapBox.AddChildToWrapBox` (`/PLATEAU-TwinLink/Widgets/WBP_TwinLinkAssetPlacementPanel.AssetPlacementWrapBox_Prop` _returnvalue) _returnvalue_3)
    (`TwinLinkAssetPlacementElement.TwinLinkAssetPlacementElementSetup` _returnvalue_3 (`.PresetID` (break `TwinLinkAssetPlacementPresetData` _array_element_2)) (`/PLATEAU-TwinLink/Widgets/WBP_TwinLinkAssetPlacementElement.AssetPlacementButton` _returnvalue_3))))