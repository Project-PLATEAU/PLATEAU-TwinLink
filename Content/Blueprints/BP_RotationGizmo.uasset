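; BP_RotationGizmo is a rotation gizmo that highlights the mesh of the active axis.
; On BeginPlay it binds to gizmo state changes, whose domain selects the X, Y or Z mesh.
; Each change first restores the previous mesh's cached materials, then caches the new mesh's materials and overrides every slot with a selection material.
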(event `self.ReceiveBeginPlay`
  (add `self.OnGizmoStateChange` (delegate `OnGizmoStateChange_Event_0`)))

(event `OnGizmoStateChange_Event_0` :!signature `self.OnGizmoStateChange`
  (params (GizmoType :type "ETwinLinkTransformationType Enum" :default "TT_NoTransform") (bTransformInProgress :type Boolean) (CurrentDomain :type "ETwinLinkTransformationDomain Enum" :default "TD_None"))
  (bind _selected_mesh (`self.Selected Mesh`))
  (bind _selected_mesh_2 (`self.Selected Mesh`))
  (`/Engine/EditorBlueprintResources/StandardMacros.IsValid` _selected_mesh
    (:`Is Valid`
      (`|ExecutionSequence`
        (:`then_0`
          (for _index (range (`PrimitiveComponent.GetNumMaterials` _selected_mesh))
            (`PrimitiveComponent.SetMaterial` (`self.Selected Mesh`) _index (`|GetArrayItem` (`self.Original Materials`) _index))))
        (:`then_1`
          (switch `ETwinLinkTransformationDomain` CurrentDomain :!label _label
            (:`TD_X_Axis`
              (set `self.Selected Mesh` (`self.X_Mesh`)))
            (:`TD_Y_Axis`
              (set `self.Selected Mesh` (`self.Y_Mesh`)))
            (:`TD_Z_Axis`
              (set `self.Selected Mesh` (`self.Z_Mesh`))))
          (set `self.Original Materials` (`MeshComponent.GetMaterials` _selected_mesh_2))
          (for _index_2 (range (`PrimitiveComponent.GetNumMaterials` _selected_mesh_2))
            (`PrimitiveComponent.SetMaterial` _selected_mesh_2 _index_2 (`self.Material for Selection`))))))
    (:`Is Not Valid`
      (goto _label))))

(fn `UserConstructionScript`)