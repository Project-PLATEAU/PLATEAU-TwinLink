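; Scene component that visualizes people flow as a heatmap decal over the PLATEAU city model of its owning BP_TwinLink.
; BeginPlay initializes the visualizer with that model, starts it inactive, then after a short delay requests automatic min/max from the server.
; Update events spawn one decal actor and dynamic material on first use, then update transform, texture, grid tiling and emissive boost.
; Active-state changes show or hide the decal.
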(event `self.ReceiveBeginPlay`
  (bind _asplateauinstanced_city_model (`self.GetCityModelFromBPTwinLink`))
  (`self.InitVisualizer` _asplateauinstanced_city_model 16)
  (`self.SetThresholdForSubdivision` 100000.0)
  (`self.RequestChangeActiveState` false)
  ;[1 1 1] BeginPlay直後に実行すると失敗するため
  (`KismetSystemLibrary.Delay` 0.5)
  ;[1 1 1] サーバーにリクエストするので結果が返るまで数フレーム掛かる。リクエストを行ったら次の処理ににうつる
  (`self.SetMaximumAndMinimumAutomatically`))

(event `self.UpdateDecalInstance`
  (params (Center :type "Vector Structure") (Scale :type "Vector Structure") (HeatmapTexture :type "Texture Object Reference") (InHeatmapWidth :type Integer) (InHeatmapHeight :type Integer) (EmissiveBoost :type "Float (single-precision)"))
  ;[1 1 1] デカールの更新を行う
  (`self.UpdateDecalInstanceBP` Center Scale HeatmapTexture InHeatmapWidth InHeatmapHeight EmissiveBoost))

(event `self.ChangeActiveState`
  (params (bIsActiveState :type Boolean))
  (bind _heatmap_actor (`self.Heatmap Actor`))
  (bind _heatmap_actor_2 (`self.Heatmap Actor`))
  ;[1 1 1] アクティブ状態が変化した
  (if bIsActiveState
    (`/Engine/EditorBlueprintResources/StandardMacros.IsValid` _heatmap_actor
      (:`Is Valid`
        (`Actor.SetActorHiddenInGame` _heatmap_actor false)))
    (else
      (`/Engine/EditorBlueprintResources/StandardMacros.IsValid` _heatmap_actor_2
        (:`Is Valid`
          (`Actor.SetActorHiddenInGame` _heatmap_actor_2 true))))))

(fn `GetCityModelFromBPTwinLink`
  (returns (`AsPLATEAUInstanced City Model` :type "PLATEAUInstancedCityModel Object Reference"))
  (bind _asbp_twin_link (cast `/PLATEAU-TwinLink/Blueprints/BP_TwinLink` (`self.GetOwner`))
    (:`then`
      (bind _asplateauinstanced_city_model (cast `PLATEAUInstancedCityModel` (`/PLATEAU-TwinLink/Blueprints/BP_TwinLink.CityModel` _asbp_twin_link))))
    (:`CastFailed`
      _))
  (return _asplateauinstanced_city_model))

(fn `UpdateDecalInstanceBP`
  (params (Center :type "Vector Structure") (Scale :type "Vector Structure") (HeatmapTexture :type "Texture Object Reference") (HeatmapWidth :type Integer) (HeatmapDepth :type Integer) (EmissiveBoost :type "Float (double-precision)"))
  (bind _heatmap_material (`self.Heatmap Material`))
  (bind (_scale_x _scale_y _scale_z) (`KismetMathLibrary.BreakVector` (`local.Scale`)))
  (bind (_scale_x_2 _scale_y_2 _scale_z_2) (`KismetMathLibrary.BreakVector` (`local.Scale`)))
  (`/Engine/EditorBlueprintResources/StandardMacros.IsValid` (`self.Heatmap Actor`)
    (:`Is Valid`
      ;[1 1 1] デカールアクターの設定
      (`Actor.K2_SetActorTransform` (`self.Heatmap Actor`) (`KismetMathLibrary.MakeTransform` (`local.Center`) (`Actor.K2_GetActorRotation` (`self.Heatmap Actor`)) (`KismetMathLibrary.MakeVector` _scale_z_2 _scale_y_2 _scale_x_2)) false true))
    (:`Is Not Valid`
      ;[1 1 1] デカールアクターの作成、設定
      (bind _returnvalue (`|SpawnActorFromClass` "/PLATEAU-TwinLink/Blueprints/BP_HeatmapDecal.BP_HeatmapDecal_C" (`KismetMathLibrary.MakeTransform` (`local.Center`) (struct) (`KismetMathLibrary.MakeVector` _scale_z _scale_y _scale_x)) "AlwaysSpawn" "MultiplyWithRoot" null null))
      (set `self.Heatmap Actor` _returnvalue)
      ;[1 1 1] マテリアルの作成
      (bind _returnvalue_2 (`KismetMaterialLibrary.CreateDynamicMaterialInstance` "/PLATEAU-TwinLink/Materials/Heatmap/M_TwinLinkHeatmapDecal_Inst.M_TwinLinkHeatmapDecal_Inst" "M_TwinLinkHeatmapDynamic" "Transient"))
      (set `self.Heatmap Material` _returnvalue_2)))
  (`MaterialInstanceDynamic.SetTextureParameterValue` _heatmap_material "HeatLevelsTexture" (`local.HeatmapTexture`))
  (`MaterialInstanceDynamic.SetScalarParameterValue` _heatmap_material "SysEmissiveBoost" (`local.EmissiveBoost`))
  ;[1 1 1] グリッド数の設定
  (`MaterialInstanceDynamic.SetScalarParameterValue` _heatmap_material "GridUTiling" (`KismetMathLibrary.Conv_IntToDouble` (`local.HeatmapWidth`)))
  (`MaterialInstanceDynamic.SetScalarParameterValue` _heatmap_material "GridVTiling" (`KismetMathLibrary.Conv_IntToDouble` (`local.HeatmapDepth`)))
  (`DecalComponent.SetDecalMaterial` (`DecalActor.Decal` (`self.Heatmap Actor`)) _heatmap_material)
  (return))