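; Scene component that detects mouse clicks on PLATEAU room areas in the 3D city model and broadcasts which one was hit.
; While active and enabled, it line-traces from the cursor, requires a PLATEAUCityObjectGroup hit whose name starts with "grp_", then fires OnClickedRoomArea with the location and object name.
; A miss prints a prompt to click a feature, and SetClickActive toggles detection.
; An older per-room GML ID lookup remains unconnected.
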(event `self.ReceiveBeginPlay`)

(event `self.LineTraceToRoom`
  (bind (_worldlocation _worlddirection) (`PlayerController.DeprojectMousePositionToWorld` (`GameplayStatics.GetPlayerController` 0)))
  ;[1 1 1] マウスクリック位置に LineTrace を飛ばします
  (if (`self.Is Active`)
    (if (`self.IsEnableLineTrace`)
      (bind (_outhit _returnvalue) (`KismetSystemLibrary.LineTraceSingle` _worldlocation (+ _worldlocation (* _worlddirection 10000000.0)) "TraceTypeQuery1"))
      (if _returnvalue
        (bind (_bblockinghit _binitialoverlap _time _distance _location _impactpoint _normal _impactnormal _physmat _hitactor _hitcomponent) (`GameplayStatics.BreakHitResult` _outhit))
        (bind _asplateaucity_object_group (cast `PLATEAUCityObjectGroup` _hitcomponent))
        (bind _returnvalue_2 (`KismetSystemLibrary.GetObjectName` _hitcomponent))
        ;[1 1 1] プレフィックスがgrp_であるかチェック
        (if (`KismetStringLibrary.EqualEqual_StrStr` (`KismetStringLibrary.GetSubstring` _returnvalue_2 0 (`KismetStringLibrary.Len` "grp_")) "grp_")
          (`self.OnClickedRoomArea` _location _returnvalue_2))
        (else
          (`KismetSystemLibrary.PrintString` "地物をクリックしてください。"))))))

(fn `SetClickActive`
  (params (IsActive :type Boolean))
  (set `self.Is Active` IsActive))