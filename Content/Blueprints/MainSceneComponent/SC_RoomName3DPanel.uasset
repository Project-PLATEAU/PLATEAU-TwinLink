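; Scene component that shows 3D name panels, apparently for rooms, by spawning one BP_3DNamePanel actor per element of its collection.
; Collection add, remove and reset events spawn or destroy panels, tracked in a map keyed by element info.
; SetupWBP runs a full Sync, which clears all panels and rebuilds them from the raw collection.
; Each panel spawns at the origin and has its name widget set up with that element's info and zero offset.
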(event `self.OnPostAddElement`
  (params (Element :type "Object Object Reference"))
  (`self.Spawn3DWidget` Element))

(event `self.OnPostRemoveElement`
  (params (Element :type "Object Object Reference"))
  (`self.Destroy3DWidget` Element))

(event `self.OnPostReset`
  (`self.Reset3DWidget`))

(fn `Destroy3DWidget`
  (params (Key :type "Object Object Reference (by ref)"))
  (bind _name3dpanels (`self.Name3DPanels`))
  (bind (_value _returnvalue) (`BlueprintMapLibrary.Map_Find` _name3dpanels Key))
  (if _returnvalue
    (`Actor.K2_DestroyActor` _value)
    (`BlueprintMapLibrary.Map_Remove` _name3dpanels Key)
    (else
      (`KismetSystemLibrary.PrintString` "Failed"))))

(fn `Reset3DWidget`
  (bind _values (`BlueprintMapLibrary.Map_Values` (`self.Name3DPanels`)))
  (for _array_element _values
    (`Actor.K2_DestroyActor` _array_element))
  (`BlueprintMapLibrary.Map_Clear` (`self.Name3DPanels`)))

(fn `Setup WBP`
  (`self.Sync`))

(fn `Spawn3DWidget`
  (params (InInfo :type "Object Object Reference"))
  (locals (Info :type "Object Object Reference"))
  (set `local.Info` InInfo)
  (bind _returnvalue (`|SpawnActorFromClass` "/PLATEAU-TwinLink/Blueprints/Widget3D/BP_3DNamePanel.BP_3DNamePanel_C" (`KismetMathLibrary.MakeTransform` (0.0 0.0 0.0)) "AlwaysSpawn" "MultiplyWithRoot" null null))
  (`BlueprintMapLibrary.Map_Add` (`self.Name3DPanels`) (`local.Info`) _returnvalue)
  (bind _aswbp_twin_link_name_3dpanel (`/PLATEAU-TwinLink/Blueprints/Widget3D/BP_3DNamePanel.GetNamePanelWidget` _returnvalue))
  (`TwinLinkInfo3DPanelBase.Setup` _aswbp_twin_link_name_3dpanel (`local.Info`) (0.0 0.0 0.0))
  (`/PLATEAU-TwinLink/Widgets/Common/WBP_TwinLinkName3DPanel.SetupWBP` _aswbp_twin_link_name_3dpanel)
  (return))

(fn `Sync`
  (`self.Reset3DWidget`)
  (bind _returnvalue (`self.GetCollectionRaw`))
  (for _array_element _returnvalue
    (`self.Spawn3DWidget` _array_element)))