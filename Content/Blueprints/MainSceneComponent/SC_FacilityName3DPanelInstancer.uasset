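; Scene component that manages the in-world 3D name panels for TwinLink facilities, reacting to element add, remove and reset events.
; Adding spawns a BP_FacilityName3DDisplay, initializes its "Info Panel Widget" with the element and moves the actor to the widget's display position.
; Actors are tracked in a map by feature ID.
; Removal destroys the matching actor but leaves its map entry, while reset destroys all actors and clears the map.
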(event `self.OnPostAddElement`
  (params (Element :type "Object Object Reference"))
  (`self.SpawnFacilityName3DPanel` Element))

(event `self.OnPostRemoveElement`
  (params (Element :type "Object Object Reference"))
  (`self.DestroyFacilityName3DPanel` Element))

(event `self.OnPostReset`
  (`self.ResetFacilityName3DPanels`))

(fn `DestroyFacilityName3DPanel`
  (params (NewParam :type "Object Object Reference"))
  (bind _astwin_link_facility_info (cast `TwinLinkFacilityInfo` NewParam))
  (bind (_value _returnvalue) (`BlueprintMapLibrary.Map_Find` (`self.ActorWidgets`) (`TwinLinkFacilityInfo.GetFeatureID` _astwin_link_facility_info)))
  (if _returnvalue
    (`Actor.K2_DestroyActor` _value)))

(fn `ResetFacilityName3DPanels`
  (bind _values (`BlueprintMapLibrary.Map_Values` (`self.ActorWidgets`)))
  (for _array_element _values
    (`Actor.K2_DestroyActor` _array_element))
  (`BlueprintMapLibrary.Map_Clear` (`self.ActorWidgets`)))

(fn `SpawnFacilityName3DPanel`
  (params (NewParam :type "Object Object Reference"))
  (locals (Widget :type "WidgetComponent Object Reference") (WidgetData :type "Object Object Reference") (Actor :type "/PLATEAU-TwinLink/Blueprints/BP_FacilityName3DDisplay Object Reference"))
  (set `local.WidgetData` NewParam)
  ;[1 1 1] アクターの生成
  (bind _returnvalue (`|SpawnActorFromClass` "/PLATEAU-TwinLink/Blueprints/BP_FacilityName3DDisplay.BP_FacilityName3DDisplay_C" (`KismetMathLibrary.MakeTransform` (0.0 4000.0 0.0)) "Undefined" "MultiplyWithRoot" null null))
  (set `local.Actor` _returnvalue)
  ;[1 1 1] 特定のウィジェットのコンポーネントの取得
  (for _array_element (`Actor.K2_GetComponentsByClass` (`local.Actor`) "/Script/UMG.WidgetComponent")
    (set `local.Widget` _array_element)
    (switch `string` (`KismetSystemLibrary.GetObjectName` (`local.Widget`))
      (:`InfoPanelWidget`
        ;[1 1 1] Widgetの設定
        (bind _aswbp_facility_name_3dpanel (cast `/PLATEAU-TwinLink/Widgets/WidgetParts/FacilityInfo/WBP_TwinLinkFacilityName3DPanel` (`WidgetComponent.GetWidget` (`local.Widget`)))
          (:`then`
            (`/PLATEAU-TwinLink/Widgets/WidgetParts/FacilityInfo/WBP_TwinLinkFacilityName3DPanel.SetupUMG` _aswbp_facility_name_3dpanel (`local.WidgetData`))
            ;[1 1 1] アクターの設定
            (`Actor.K2_SetActorLocation` (`local.Actor`) (`TwinLinkFacilityInfo3DPanelBase.GetDisplayPosition` _aswbp_facility_name_3dpanel) false false)
            ;[1 1 1] 管理コレクションに追加
            (`BlueprintMapLibrary.Map_Add` (`self.ActorWidgets`) (`TwinLinkFacilityInfo.GetFeatureID` (`TwinLinkFacilityInfo3DPanelBase.GetData` _aswbp_facility_name_3dpanel)) (`local.Actor`)))
          (:`CastFailed`
            (`KismetSystemLibrary.PrintString` "Failed cast")))))))